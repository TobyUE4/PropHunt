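; Player Blueprint for a prop mechanic, handling the health HUD and the input that turns the player into a prop.
; BeginPlay creates the PlayerHUD widget, adds it to the viewport and fills its health bar and text from the health getters.
; The Become Prop input calls BecomeProp, then reruns that same health refresh.
; The HUD updates only at those two moments, with no Tick or binding.
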(event EventBeginPlay
  (bind _returnvalue (UserInterface|CreateWidget "/Game/UI/HUD/PlayerHUD.PlayerHUD_C"))
  (bind _output_get (Variables|Default|SetHUD%20Widget _returnvalue))
  (UserInterface|Viewport|AddtoViewport _output_get 0)
  (bind _returnvalue_2 (Class|PropPC|GetHealthasPercent))
  (Progress|SetPercent (Variables|/Game/UI/HUD/PlayerHUD.PlayerHUD_C|GetHealth_Bar (Variables|Default|GetHUD%20Widget)) _returnvalue_2)
  (bind _returnvalue_3 (Class|PropPC|GetHealthPoints))
  (Rendering|Components|TextRender|SetText (Variables|/Game/UI/HUD/PlayerHUD.PlayerHUD_C|GetHealth_Text (Variables|Default|GetHUD%20Widget)) (Utilities|Text|ToText(String) (Utilities|String|Append "Health: " (Utilities|String|ToString(Integer) _returnvalue_3) "%"))))

(event EventTick
  (params (DeltaSeconds :type Float%20%28single-precision%29)))

(event Input|ActionEvents|InputActionBecomeProp
  (params (Key :type Key%20Structure :default "AnyKey"))
  (:Pressed
    (Class|PropPC|BecomeProp)
    (bind _returnvalue (Class|PropPC|GetHealthasPercent))
    (Progress|SetPercent (Variables|/Game/UI/HUD/PlayerHUD.PlayerHUD_C|GetHealth_Bar (Variables|Default|GetHUD%20Widget)) _returnvalue)
    (bind _returnvalue_2 (Class|PropPC|GetHealthPoints))
    (Rendering|Components|TextRender|SetText (Variables|/Game/UI/HUD/PlayerHUD.PlayerHUD_C|GetHealth_Text (Variables|Default|GetHUD%20Widget)) (Utilities|Text|ToText(String) (Utilities|String|Append "Health: " (Utilities|String|ToString(Integer) _returnvalue_2) "%")))))

(fn ConstructionScript)