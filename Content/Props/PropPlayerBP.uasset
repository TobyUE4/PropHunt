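; Player-controlled prop, with input for camera, movement, rotation and jumping.
; Look axes rotate a spring arm and azimuth gimbal, while move and rotate axes apply local offsets to CurrentProp without sweeping.
; Jump uses a timeline to push the prop upward with sweep, gated by HasJumped until a short delay after it finishes.
; Become Prop and Interact are placeholders that only print text.
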(event EventBeginPlay)

(event EventActorBeginOverlap
  (params (OtherActor :type Actor%20Object%20Reference)))

(event EventTick
  (params (DeltaSeconds :type Float%20%28single-precision%29)))

(event Input|ActionEvents|InputActionBecomeProp
  (params (Key :type Key%20Structure :default "AnyKey"))
  (:Pressed
    (Development|PrintText "Prop swap")))

(event Input|ActionEvents|InputActionInteract
  (params (Key :type Key%20Structure :default "AnyKey"))
  (:Pressed
    (Development|PrintText "Interaction")))

(event Input|ActionEvents|InputActionJump
  (params (Key :type Key%20Structure :default "AnyKey"))
  ;[1 1 1] Jump Controls
  (:Pressed
    (if (not (Variables|Default|GetHasJumped))
      (Timeline|Jump%20Timeline PlayFromStart
        (:Update
          (Class|SceneComponent|AddLocalTransform (Variables|Default|GetCurrentProp) (Math|Transform|MakeTransform (Math|Vector|MakeVector 0.0 0.0 15.0)) true false)
          (Variables|Default|SetHasJumped true))
        (:Finished
          (Utilities|FlowControl|Delay 1.0)
          (Variables|Default|SetHasJumped false))))))

(event Input|AxisEvents|InputAxisLookUp/Down
  (params (AxisValue :type Float%20%28single-precision%29))
  ;[1 1 1] Camera Controls
  (Transformation|AddLocalRotation (Variables|Default|GetSpringArm) (Math|Rotator|MakeRotator 0.0 AxisValue 0.0) false false))

(event Input|AxisEvents|InputAxisLookRight/Left
  (params (AxisValue :type Float%20%28single-precision%29))
  ;[1 1 1] Camera Controls
  (Transformation|AddLocalRotation (Variables|Default|GetAzimuth%20Gimbal) (Math|Rotator|MakeRotator 0.0 0.0 AxisValue) false false))

(event Input|AxisEvents|InputAxisRotateProp
  (params (AxisValue :type Float%20%28single-precision%29))
  ;[1 1 1] Rotation Controls
  (Transformation|AddLocalRotation (Variables|Default|GetCurrentProp) (Math|Rotator|MakeRotator 0.0 0.0 AxisValue) false false))

(event Input|AxisEvents|InputAxisMoveForwards
  (params (AxisValue :type Float%20%28single-precision%29))
  ;[1 1 1] Movement Controls
  (Class|SceneComponent|AddLocalTransform (Variables|Default|GetCurrentProp) (Math|Transform|MakeTransform (Math|Vector|MakeVector AxisValue 0.0 0.0)) false false))

(event Input|AxisEvents|InputAxisMoveBackwards
  (params (AxisValue :type Float%20%28single-precision%29))
  ;[1 1 1] Movement Controls
  (Class|SceneComponent|AddLocalTransform (Variables|Default|GetCurrentProp) (Math|Transform|MakeTransform (Math|Vector|MakeVector AxisValue 0.0 0.0)) false false))

(event Input|AxisEvents|InputAxisStrafeLeft
  (params (AxisValue :type Float%20%28single-precision%29))
  ;[1 1 1] Movement Controls
  (Class|SceneComponent|AddLocalTransform (Variables|Default|GetCurrentProp) (Math|Transform|MakeTransform (Math|Vector|MakeVector 0.0 AxisValue 0.0)) false false))

(event Input|AxisEvents|InputAxisStrafeRight
  (params (AxisValue :type Float%20%28single-precision%29))
  ;[1 1 1] Movement Controls
  (Class|SceneComponent|AddLocalTransform (Variables|Default|GetCurrentProp) (Math|Transform|MakeTransform (Math|Vector|MakeVector 0.0 AxisValue 0.0)) false false))

(fn ConstructionScript)